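; Gameplay ability for Aura's Electrocute lightning spell, so far handling only targeting, cursor visibility and hold-to-channel input.
; On activation, a TargetDataUnderMouse task supplies the hit result, which is stored along with the owning player controller.
; The mouse cursor hides while input is held; WaitInputRelease restores it and ends the ability.
; The event graph contains no damage or effect logic.
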(event Ability|EventActivateAbility
  ;[0.2403 0.18 1] Store Mouse Data Variables
  (bind _datahandle (|TargetDataUnderMouse)
    (:ValidData
      (Class|AuraBeamSpell|StoreMouseDataInfo (Ability|TargetData|GetHitResultfromTargetData _datahandle))
      (Class|AuraBeamSpell|StoreOwnerPlayerController)
      (Utilities|FlowControl|Sequence
        (:then_0
          (Variables|/Script/Engine.PlayerController|SetbShowMouseCursor (Variables|Default|GetOwnerPlayerController) false))
        (:then_1
          (Ability|Tasks|WaitInputRelease false
            (:OnRelease
              (Variables|/Script/Engine.PlayerController|SetbShowMouseCursor (Variables|Default|GetOwnerPlayerController) true)
              (Ability|EndAbility))))))))